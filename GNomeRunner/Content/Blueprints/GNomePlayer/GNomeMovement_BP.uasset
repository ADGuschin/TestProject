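; GNomeMovement_BP is a player gnome Blueprint that handles jumping, health and survival time.
; The Jump input plays a gnome sound at the current location, then jumps.
; Damage events subtract from Health, which the construction script initializes.
; Tick calls the player-died dispatcher on every frame that Health is depleted, and otherwise updates the time elapsed since BeginPlay.
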(event Custom|Damage
  (params (Damage :type Float%20%28single-precision%29))
  (Variables|Default|SetHealth (- (Variables|Default|GetHealth) Damage)))

(event EventTick
  (params (DeltaSeconds :type Float%20%28single-precision%29))
  (if (<= (Variables|Default|GetHealth) 0.0)
    (Default|CallPlayerDiedEventDispatcher)
    (else
      (Variables|Default|SetTime (- (Math|DateTime|Now) (Variables|Default|GetStartTime))))))

(event EventBeginPlay
  (Variables|Default|SetStartTime (Math|DateTime|Now)))

(event Input|ActionEvents|InputActionJump
  (params (Key :type Key%20Structure :default "None"))
  (:Pressed
    (bind _location (CallFunction|GetCurrentLocation))
    (Audio|PlaySoundatLocation "/Game/Meshes/GNomeSexySound.GNomeSexySound" (.location _location) "0, 0, 0" 1.0 1.0 0.0 0 0 0)
    (Character|Jump)))

(fn ConstructionScript
  (Variables|Default|SetHealth 1e+02))

(fn GetZ
  (return (.z (.location (Transformation|GetActorTransform)))))

(fn GetCurrentLocation
  (return (Transformation|GetActorTransform)))