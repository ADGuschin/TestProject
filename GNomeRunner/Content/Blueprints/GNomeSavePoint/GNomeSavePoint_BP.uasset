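; GNomeSavePoint_BP is a save point actor that triggers once when the player's GNomeMovement_BP character comes near it.
; Each Tick until triggered, it casts its root's owner to itself and polls horizontal distance to the player instead of using an overlap volume.
; Within range it calls CallSavePointEvent, whose handling is not in this graph, and sets Checked so it does not fire again.
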(event EventTick
  (params (DeltaSeconds :type Float%20%28single-precision%29))
  (if (not (Variables|Default|GetChecked))
    (bind _asgnome_save_point_bp (Utilities|Casting|CastToGNomeSavePoint_BP (Components|GetOwner (Variables|Default|GetDefaultSceneRoot)))
      (:then
        (bind _asgnome_movement_bp (Utilities|Casting|CastToGNomeMovement_BP (Game|GetPlayerCharacter 0)))
        (if (<= (Transformation|GetHorizontalDistanceTo _asgnome_save_point_bp _asgnome_movement_bp) 1.5e+02)
          (Default|CallSavePointEvent)
          (Variables|Default|SetChecked true)))
      (:CastFailed
        (Development|PrintString "GNomeSavePoint_BP cast failed")))))

(fn ConstructionScript)