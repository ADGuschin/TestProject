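; GNome save point character that approaches the player, triggers a save point event, then roams between destinations.
; Until activated, Tick checks horizontal distance to the player and, within close range, starts an AI move toward them, calling the save event after a short delay.
; It then changes state and starts Checked, which loops: move to a destination, play a sound on success, pick a random next one, and wait a random time.
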(event Custom|Checked
  (if (Utilities|Enum|Equal(Enum) (Variables|Default|GetState) "NewEnumerator1")
    (AI|AIMoveTo self "0, 0, 0" (Utilities|Array|Get(acopy) (Variables|Default|GetDestinations) (Variables|Default|GetTarget)) 5.0 false :!label _label
      (:OnSuccess
        (Audio|PlaySoundatLocation "/Game/Meshes/GNomeSexySound.GNomeSexySound" (Transformation|GetActorLocation) "0, 0, 0" 1.0 1.0 0.0 0 0 0)
        (Variables|Default|SetTarget (Math|Random|RandomIntegerinRange 0 (- (Utilities|Array|Length (Variables|Default|GetDestinations)) 1)))
        (Utilities|FlowControl|Delay (+ (Math|Float|%(Float) (Math|Random|RandomFloat) 3e+01) 5.0))
        (goto _label)))))

(event EventTick
  (params (DeltaSeconds :type Float%20%28single-precision%29))
  (bind _returnvalue (Game|GetPlayerCharacter 0))
  (if (not (Utilities|Enum|Equal(Enum) (Variables|Default|GetState) "NewEnumerator1"))
    (bind _asgnome_save_point_char_bp (Utilities|Casting|CastToGNomeSavePointChar_BP (Class|CharacterMovementComponent|GetCharacterOwner (Variables|Character|GetCharacterMovement)))
      (:then
        (bind _asgnome_movement_bp (Utilities|Casting|CastToGNomeMovement_BP _returnvalue))
        (if (<= (Transformation|GetHorizontalDistanceTo _asgnome_save_point_char_bp _asgnome_movement_bp) 1.5e+02)
          (AI|AIMoveTo self "0, 0, 0" _returnvalue 5.0 false
            (:then
              (Utilities|FlowControl|Delay 2.0)
              (Default|CallSavePointEvent)
              (Variables|Default|SetState "NewEnumerator1")
              (CallFunction|Checked)))))
      (:CastFailed
        (Development|PrintString "GNomeSavePoint_BP cast failed")))))

(fn ConstructionScript)